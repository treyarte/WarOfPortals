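; BP_Cube is an actor that travels along the spline of a BP_SplinePath actor, found at BeginPlay.
; The MoveObject event plays a timeline at a rate of 1/TimeToComplete, mapping its track to distance along the spline length.
; Each update sets the actor's transform from the spline's world-space location and local-space rotation.
; The construction script also looks up the path but discards the result.
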(event Custom|Move%20Object
  (bind _newvar (Variables|Default|GetNewVar))
  (bind _spline (Variables|/Game/Blueprints/BP_SplinePath.BP_SplinePath_C|GetSpline _newvar))
  (Components|Timeline|SetPlayRate (Variables|Default|GetT_MoveObject) (/ 1.0 (Variables|Default|GetTimeToComplete)))
  (bind _movetrack (Timeline|T_MoveObject Play)
    (:Update
      (Transformation|SetActorTransform (Math|Transform|MakeTransform (Spline|GetLocationatDistanceAlongSpline _spline (Math|Float|Lerp 0.0 (Spline|GetSplineLength (Variables|/Game/Blueprints/BP_SplinePath.BP_SplinePath_C|GetSpline (Variables|Default|GetNewVar))) _movetrack) "World") (Spline|GetRotationatDistanceAlongSpline _spline (Math|Float|Lerp 0.0 (Spline|GetSplineLength (Variables|/Game/Blueprints/BP_SplinePath.BP_SplinePath_C|GetSpline (Variables|Default|GetNewVar))) _movetrack) "Local") "1.000000,1.000000,1.000000")))))

(event EventBeginPlay
  (bind _returnvalue (Actor|GetActorOfClass "/Game/Blueprints/BP_SplinePath.BP_SplinePath_C"))
  (Variables|Default|SetNewVar _returnvalue))

(fn ConstructionScript
  (Actor|GetActorOfClass "/Game/Blueprints/BP_SplinePath.BP_SplinePath_C"))