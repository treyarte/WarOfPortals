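; BP_SplinePath moves an array of enemies along a spline in a looping timeline.
; Timeline alpha drives each actor's location and rotation, with an index-based distance offset that wraps at the spline length.
; An enemy whose world Y drops to or below the second-to-last spline point's gets its reached-end event and Death called.
; Destroyed enemies are removed from the array through bound OnDestroyed events.
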(event Custom|PlayTimeLine
  (bind _spline (Variables|Default|GetSpline))
  (bind _spline_2 (Variables|Default|GetSpline))
  (bind _returnvalue (Spline|GetSplineLength _spline))
  (bind _alpha (Timeline|Timeline PlayFromStart)
    (:Update
      (for (_array_element _array_index) (Variables|Default|GetActors)
        (bind _output_get (Variables|Default|SetDistance%20Along%20Spline (+ (Math|Float|Lerp 0.0 (Spline|GetSplineLength (Variables|Default|GetSpline)) _alpha) (* _array_index (Variables|Default|GetOffset%20Between%20Actors)))))
        (if (> _output_get _returnvalue)
          (Variables|Default|SetDistance%20Along%20Spline (- (Variables|Default|GetDistance%20Along%20Spline) _returnvalue)))
        (Transformation|SetActorLocationAndRotation _array_element (Spline|GetLocationatDistanceAlongSpline _spline_2 (Variables|Default|GetDistance%20Along%20Spline) "World") (Spline|GetRotationatDistanceAlongSpline _spline_2 (Variables|Default|GetDistance%20Along%20Spline) "World"))
        (CallFunction|CheckEndOfSpline _array_element)))
    (:Finished
      (CallFunction|PlayTimeLine))))

(event Custom|Death
  (params (DestroyedActor :type Actor%20Object%20Reference))
  (bind _asbp_enemy (Utilities|Casting|CastToBP_Enemy DestroyedActor))
  (bind _returnvalue (Utilities|Array|RemoveItem (Variables|Default|GetActors) _asbp_enemy))
  (if _returnvalue
    (Development|PrintString "REMOVED")
    (else
      (Development|PrintString "NOPE"))))

(event EventBeginPlay
  (Components|Timeline|SetPlayRate (Variables|Default|GetTimeline) (/ 1.0 (Variables|Default|GetTimeline%20Length)))
  (CallFunction|PlayTimeLine)
  (for _array_element (Variables|Default|GetActors)
    (Game|BindEventtoOnDestroyed _array_element (delegate Custom|Death))))

(fn ConstructionScript)

(fn CheckEndOfSpline
  (params (Current_Enemy :type BP%20Enemy%20Object%20Reference))
  (bind _returnvalue (CallFunction|GetLastSplinePointLoc))
  (if (<= (.Y (Math|Vector|BreakVector (Transformation|GetActorLocation Current_Enemy))) (.Y (Math|Vector|BreakVector _returnvalue)))
    (Default|ReachedEndEvent Current_Enemy)
    (Default|Death Current_Enemy)))

(fn GetLastSplinePointLoc
  (return (Spline|GetLocationatSplinePoint (Variables|Default|GetSpline) (- (Spline|GetNumberOfSplinePoints (Variables|Default|GetSpline)) 2) "World")))