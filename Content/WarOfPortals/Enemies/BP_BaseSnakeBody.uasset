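; Base snake enemy body segment with its own health, shown on left and right text displays.
; Damage, healing and health queries forward to BPC_DamageSystem, whose death, block and damage-response events are bound in the construction script.
; A hit updates both texts and briefly flashes the cube's material red before setting it back to blue.
; Death enables mesh physics, calls OnSnakeBodyBreak and immediately destroys the actor, while a block only prints a message.
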(event Custom|Blocked
  (params (CanBeParried :type Boolean))
  (Development|PrintString "BLocked"))

(event Custom|Death
  (bind _mesh (Variables|Character|GetMesh))
  (Physics|SetSimulatePhysics _mesh true)
  (Collision|SetCollisionEnabled _mesh "QueryAndPhysics")
  (Default|CallOnSnakeBodyBreak)
  (Actor|DestroyActor))

(event Custom|DamageResponse
  (params (DamageResponse :type E_DamageResponse%20Enum :default "NewEnumerator0"))
  (CallFunction|SetHealthText (Variables|Default|GetHealthLeftTxt) (Variables|Default|GetHealthRightTxt))
  (Rendering|Material|SetMaterial (Variables|Default|GetSM_ChamferCube) 0 "/Game/WarOfPortals/Materials/MI_DamagedRed.MI_DamagedRed")
  (Utilities|FlowControl|Delay 0.1)
  (Rendering|Material|SetMaterial (Variables|Default|GetSM_ChamferCube) 0 "/Game/LevelPrototyping/Materials/MI_Solid_Blue.MI_Solid_Blue"))

(fn ConstructionScript
  (bind _bpc_damagesystem (Variables|Default|GetBPC_DamageSystem))
  (CallFunction|SetHealthText (Variables|Default|GetHealthLeftTxt) (Variables|Default|GetHealthRightTxt))
  (EventDispatchers|BindEventtoOnDeath _bpc_damagesystem (EventDispatchers|CreateEvent :!event Custom|Death))
  (EventDispatchers|BindEventtoOnBlocked _bpc_damagesystem (EventDispatchers|CreateEvent :!event Custom|Blocked))
  (EventDispatchers|BindEventtoOnDamageResponse _bpc_damagesystem (EventDispatchers|CreateEvent :!event Custom|DamageResponse)))

(fn SetHealthText
  (params (self2 :type Text%20Render%20Component%20Object%20Reference) (self1 :type Text%20Render%20Component%20Object%20Reference))
  (Rendering|Components|TextRender|SetText self2 (Utilities|Text|ToText(Float) (Variables|/Game/DamageSystem/BPC_DamageSystem.BPC_DamageSystem_C|GetHealth (Variables|Default|GetBPC_DamageSystem)) "HalfToEven")))

(fn GetCurrentHealth
  (return (Variables|/Game/DamageSystem/BPC_DamageSystem.BPC_DamageSystem_C|GetHealth (Variables|Default|GetBPC_DamageSystem))))

(fn GetMaxHealth
  (return (Variables|/Game/DamageSystem/BPC_DamageSystem.BPC_DamageSystem_C|GetMaxHealth (Variables|Default|GetBPC_DamageSystem))))

(fn Heal
  (params (Amount :type Float%20%28double-precision%29))
  (Default|Heal (Variables|Default|GetBPC_DamageSystem) Amount)
  (return 0.0))

(fn TakeDamage
  (params (DamageInfo :type S%20Damage%20Info%20Structure))
  (bind _wasdamaged (Default|TakeDamage (Variables|Default|GetBPC_DamageSystem) DamageInfo))
  (return _wasdamaged))