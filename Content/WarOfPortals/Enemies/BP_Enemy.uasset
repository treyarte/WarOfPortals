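; Enemy Blueprint for War of Portals that shows a health widget and damages the player by its remaining health on reaching the end.
; A damage system component holds health, with damage and health functions forwarding to it, though Heal always passes zero.
; The construction script seeds health and binds death, blocked and damage response events.
; Death ragdolls the mesh; the other responses only print debug text.
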(event Custom|Blocked
  (params (CanBeParried :type Boolean))
  (Development|PrintString "BLocked"))

(event Custom|Death
  (bind _mesh (Variables|Default|GetMesh))
  (Physics|SetSimulatePhysics _mesh true)
  (Collision|SetCollisionEnabled _mesh "QueryAndPhysics"))

(event Custom|ReachedEnd_Event
  (Development|PrintString "I reached the end")
  (Game|Damage|ApplyDamage (Game|Player|GetPlayerPawn 0) (Variables|/Game/DamageSystem/BPC_DamageSystem.BPC_DamageSystem_C|GetHealth (Variables|Default|GetBPC_DamageSystem)) 0 0))

(event Custom|DamageResponse
  (params (DamageResponse :type E_DamageResponse%20Enum :default "NewEnumerator0"))
  (Development|PrintString (Utilities|String|EnumtoString DamageResponse)))

(event EventBeginPlay
  (bind _returnvalue (UserInterface|CreateWidget "/Game/WarOfPortals/Ui/W_EnemyHealth.W_EnemyHealth_C" 0 self))
  (UserInterface|SetWidget (Variables|Default|GetHealthText) _returnvalue))

(fn ConstructionScript
  (bind _bpc_damagesystem (Variables|Default|GetBPC_DamageSystem))
  (Variables|/Game/DamageSystem/BPC_DamageSystem.BPC_DamageSystem_C|SetHealth _bpc_damagesystem (Variables|Default|GetHealth))
  (EventDispatchers|BindEventtoOnDeath _bpc_damagesystem (EventDispatchers|CreateEvent :!event Custom|Death))
  (EventDispatchers|BindEventtoOnBlocked _bpc_damagesystem (EventDispatchers|CreateEvent :!event Custom|Blocked))
  (EventDispatchers|BindEventtoOnDamageResponse _bpc_damagesystem (EventDispatchers|CreateEvent :!event Custom|DamageResponse)))

(fn GetCurrentHealth
  (return (Variables|/Game/DamageSystem/BPC_DamageSystem.BPC_DamageSystem_C|GetHealth (Variables|Default|GetBPC_DamageSystem))))

(fn GetMaxHealth
  (return (Variables|/Game/DamageSystem/BPC_DamageSystem.BPC_DamageSystem_C|GetMaxHealth (Variables|Default|GetBPC_DamageSystem))))

(fn Heal
  (params (Amount :type Float%20%28double-precision%29))
  (Default|Heal (Variables|Default|GetBPC_DamageSystem) 0.0)
  (return 0.0))

(fn TakeDamage
  (params (DamageInfo :type S%20Damage%20Info%20Structure))
  (bind _wasdamaged (Default|TakeDamage (Variables|Default|GetBPC_DamageSystem) DamageInfo))
  (return _wasdamaged))