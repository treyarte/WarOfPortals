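; Base snake enemy body part that damages the player on contact and can be destroyed.
; A capsule overlap with the player pawn applies damage equal to the part's current damage-system Health.
; Damage response briefly flashes the mesh red before restoring blue, and death destroys the actor.
; A separate DealDamage function sends fixed damage to a hit actor through TakeDamageMessage, while SetHealthText is empty.
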(event OnComponentBeginOverlap(CapsuleComponent)
  (params (OverlappedComponent :type Primitive%20Component%20Object%20Reference) (OtherActor :type Actor%20Object%20Reference) (OtherComp :type Primitive%20Component%20Object%20Reference) (OtherBodyIndex :type Integer) (bFromSweep :type Boolean) (SweepResult :type Hit%20Result%20Structure%20%28by%20ref%29))
  (if (== OtherActor (Game|Player|GetPlayerPawn 0))
    (Game|Damage|ApplyDamage OtherActor (Variables|/Game/DamageSystem/BPC_DamageSystem.BPC_DamageSystem_C|GetHealth (Variables|Default|GetBPC_DamageSystem)) 0 0)))

(event EventDeath
  (Actor|DestroyActor))

(event EventDamageResponse
  (params (DamageResponse :type E_DamageResponse%20Enum :default "NewEnumerator0"))
  (Rendering|Material|SetMaterial (Variables|Character|GetMesh) 0 "/Game/WarOfPortals/Materials/MI_DamagedRed.MI_DamagedRed")
  (Utilities|FlowControl|Delay 0.2)
  (Rendering|Material|SetMaterial (Variables|Character|GetMesh) 0 "/Game/LevelPrototyping/Materials/MI_Solid_Blue.MI_Solid_Blue"))

(fn ConstructionScript
  (|CallParentFunction))

(fn SetHealthText
  (params (self2 :type Text%20Render%20Component%20Object%20Reference) (self1 :type Text%20Render%20Component%20Object%20Reference)))

(fn DealDamage
  (params (Hit :type Hit%20Result%20Structure))
  (Class|BPIDamagable|TakeDamage(Message) (.HitActor (Collision|BreakHitResult Hit)) (Utilities|Struct|MakeS_DamageInfo 1e+01 "NewEnumerator1" "NewEnumerator1")))